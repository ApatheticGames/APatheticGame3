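; BP_PIckUpActor is a world pickup that gives an item to the player's inventory on overlap.
; Its sphere's begin overlap casts the other actor to ThirdPersonCharacter and calls AddItem on that character's InventoryReference with ItemToAdd and Amount.
; On success it destroys itself if no rest remains; otherwise it stays and sets Amount to zero rather than to the leftover.
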(event OnComponentBeginOverlap(Sphere)
  (params (OverlappedComponent :type Primitive%20Component%20Object%20Reference) (OtherActor :type Actor%20Object%20Reference) (OtherComp :type Primitive%20Component%20Object%20Reference) (OtherBodyIndex :type Integer) (bFromSweep :type Boolean) (SweepResult :type Hit%20Result%20Structure%20%28by%20ref%29))
  (bind _asthird_person_character (Utilities|Casting|CastToThirdPersonCharacter OtherActor))
  (Utilities|IsValid (Variables|/Game/ThirdPersonCPP/Blueprints/ThirdPersonCharacter.ThirdPersonCharacter_C|GetInventoryReference _asthird_person_character)
    (:Is%20Valid
      (bind (_success _rest) (Default|AddItem (Variables|/Game/ThirdPersonCPP/Blueprints/ThirdPersonCharacter.ThirdPersonCharacter_C|GetInventoryReference _asthird_person_character) (Variables|Default|GetItemToAdd) (Variables|Default|GetAmount)))
      (if _success
        (if (> _rest 0)
          (Variables|Default|SetAmount 0)
          (else
            (Actor|DestroyActor)))))))

(fn ConstructionScript)