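; Slot-based inventory that stores item classes with amounts in an array sized on BeginPlay.
; AddItem reads the item's stackable default, searches for stacks or empty slots, and recurses to place overflow, returning success and the remainder.
; Query functions report slot contents, though IsSlotEmpty always returns false and GetItemInfoAtIndex always reads slot zero.
; The wiring is unfinished: stack merging never runs, and non-stackable items are stored as BP_MasterItem.
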(event EventBeginPlay
  (Utilities|Array|Resize (Variables|Default|GetSlots) (Variables|Default|GetAmountOfSlots)))

(fn ConstructionScript)

(fn IsSlotEmpty
  (params (Index :type Integer))
  (return false))

(fn GetItemInfoatIndex
  (params (Index :type Integer))
  (bind _slots (Variables|Default|GetSlots))
  (bind _output (Utilities|Array|Get(acopy) _slots))
  (bind (_itemclass _amount) (Utilities|Struct|BreakInventorySlot _output))
  (if (Utilities|IsValidClass _itemclass)
    (return false (Utilities|GetClassDefaults _itemclass) _amount)
    (else
      (return true "" 0))))

(fn SearchEmptySLot
  (bind (_array_element _array_index) (Utilities|Array|ForEachLoopwithBreak (Variables|Default|GetSlots) :!label _label)
    (:LoopBody
      (if (not (Utilities|IsValidClass (.ItemClass (Utilities|Struct|BreakInventorySlot _array_element))))
        (LocalVariables|SetLocal true)
        (LocalVariables|SetLocalIndex _array_index)
        (goto _label Break)))
    (:Completed
      (return (LocalVariables|GetLocal) (LocalVariables|GetLocalIndex)))))

(fn SearchFreeStack
  (params (ItemClass :type BP%20Master%20Item%20Class%20Reference))
  (bind (_array_element _array_index) (Utilities|Array|ForEachLoopwithBreak (Variables|Default|GetSlots) :!label _label)
    (:LoopBody
      (if (Utilities|IsValidClass (.ItemClass (Utilities|Struct|BreakInventorySlot _array_element)))
        (if (and (== (.ItemClass (Utilities|Struct|BreakInventorySlot _array_element)) ItemClass) (< (.Amount (Utilities|Struct|BreakInventorySlot _array_element)) (Variables|Default|GetMaxStackSize)))
          (LocalVariables|SetBool false)
          (goto _label Break))))
    (:Completed
      (return (LocalVariables|GetBool) (LocalVariables|GetLocalIndex)))))

(fn AddItem
  (params (ItemClass :type BP%20Master%20Item%20Class%20Reference) (AmountOfItems :type Integer))
  (bind (_success _index) (CallFunction|SearchEmptySLot))
  (LocalVariables|SetLocalClass ItemClass)
  (LocalVariables|SetAmount AmountOfItems)
  (if (.CanBeStacked (Utilities|Struct|BreakItemInfo (Utilities|GetClassDefaults ItemClass)))
    (if (.Success (CallFunction|SearchFreeStack (LocalVariables|GetLocalClass)))
      (LocalVariables|SetFoundIndex (.Index (CallFunction|SearchFreeStack (LocalVariables|GetLocalClass))))
      (elif (.Success (CallFunction|SearchEmptySLot))
        (if (> (LocalVariables|GetAmount) (Variables|Default|GetAmountOfSlots))
          (Utilities|Array|SetArrayElem (Variables|Default|GetSlots) (stale _output_get) (Utilities|Struct|MakeInventorySlot (LocalVariables|GetLocalClass) (Variables|Default|GetMaxStackSize)))
          (bind _rest (CallFunction|AddItem (LocalVariables|GetLocalClass) (- (LocalVariables|GetAmount) (Variables|Default|GetMaxStackSize))))
          (return true _rest)
          (else
            (Utilities|Array|SetArrayElem (Variables|Default|GetSlots) (LocalVariables|GetFoundIndex) (Utilities|Struct|MakeInventorySlot (LocalVariables|GetLocalClass) (LocalVariables|GetAmount)))
            (return true 0)))
        (else
          (return false (LocalVariables|GetAmount)))))
    (elif _success
      (LocalVariables|SetFoundIndex _index)
      (Utilities|Array|SetArrayElem (Variables|Default|GetSlots) _index (Utilities|Struct|MakeInventorySlot "/Game/InventorySystem2/Blueprints/ItemClasses/BP_MasterItem.BP_MasterItem_C" 1))
      (if (> (LocalVariables|GetAmount) 1)
        (bind _rest_2 (CallFunction|AddItem (LocalVariables|GetLocalClass) (- (LocalVariables|GetAmount) 1)))
        (return true _rest_2)
        (else
          (return true 0)))
      (else
        (return false (LocalVariables|GetAmount))))))

(fn GetAmountatIndex
  (params (Index :type Integer))
  (return (.Amount (Utilities|Struct|BreakInventorySlot (Utilities|Array|Get(acopy) (Variables|Default|GetSlots) Index)))))